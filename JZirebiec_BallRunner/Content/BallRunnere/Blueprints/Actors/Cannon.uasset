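; Cannon actor for BallRunnere that repeatedly spawns Enemy actors as projectiles.
; After a two-second delay on BeginPlay, it waits FireRate, spawns a scaled Enemy at the Spawn component, then plays the CannonFire timeline and loops when it finishes.
; Timeline updates animate the cannon's relative Y through a Lerp toward zero, which uses the cannon's world Y as alpha.
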(event EventBeginPlay
  (Utilities|FlowControl|Delay 2.0)
  (Utilities|FlowControl|Delay (Variables|cannon|Getfire%20rate) :!label _label)
  (CallFunction|SpawnEnemy)
  (bind _cannon_y (Timeline|Cannon%20Fire PlayFromStart)
    (:Update
      (CallFunction|CannonReSet _cannon_y))
    (:Finished
      (goto _label))))

(fn ConstructionScript)

(fn SpawnEnemy
  (bind _spawn (Variables|Default|Getspawn))
  (Game|SpawnActorfromClass "/Game/BallRunnere/Blueprints/Actors/Projectiles/Enemy.Enemy_C" (Math|Transform|MakeTransform (Transformation|GetWorldLocation _spawn) (Transformation|GetWorldRotation _spawn) (Math|Conversions|ToVector(Float) (Variables|cannon|GetProjectile%20Scale))) "AlwaysSpawn" 0 0))

(fn CannonReSet
  (params (A :type Float%20%28single-precision%29))
  (Transformation|SetRelativeLocation (Variables|Default|GetCannon) (Math|Vector|MakeVector 0.0 (Math|Float|Lerp A 0.0 (.y (Transformation|GetWorldLocation (Variables|Default|GetCannon)))) 0.0) false false))