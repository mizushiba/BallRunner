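; Collectable crystal actor for BallRunnere that is pulled into the player and vanishes when the player pawn overlaps it.
; On overlap it caches its location, scale and point light intensity, then plays a timeline with separate curves for each.
; Each update lerps it toward the player's current position, shrinks it to zero and fades the light, then the actor destroys itself when finished.
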(event Collision|EventActorBeginOverlap
  (params (OtherActor :type Actor%20Object%20Reference))
  (Utilities|IsPlayer OtherActor
    (:is%20player
      (CallFunction|StartCrystalValues)
      (bind (_direction _smoothlerpalpha _sacle_in_time _light_flicker) (Timeline|TL_BlendAlpha Play)
        (:Update
          (CallFunction|CrystalLocation _smoothlerpalpha)
          (CallFunction|CrystalScale _sacle_in_time)
          (CallFunction|CrystalLightIntensity _light_flicker))
        (:Finished
          (Actor|DestroyActor))))))

(fn ConstructionScript)

(fn MovetoPlayer
  (params (Alpha :type Float%20%28single-precision%29))
  (return (Math|Vector|Lerp(Vector) (Variables|Default|GetLerp%20start%20Location) (Transformation|GetActorLocation (Game|Player|GetPlayerPawn 0)) Alpha)))

(fn StartCrystalValues
  (Variables|Default|SetLerp%20start%20Location (Transformation|GetActorLocation))
  (Variables|Default|SetLerpStartScale (Transformation|GetActorScale3D))
  (Variables|Default|SetLerp%20Start%20Intensity (Variables|/Script/Engine.LightComponentBase|GetIntensity (Variables|Default|GetPointLight))))

(fn CrystalLocation
  (params (Alpha :type Float%20%28single-precision%29))
  (Transformation|SetActorLocation (Math|Vector|Lerp(Vector) (Variables|Default|GetLerp%20start%20Location) (Transformation|GetActorLocation (Game|Player|GetPlayerPawn 0)) Alpha) false false))

(fn CrystalScale
  (params (Alpha :type Float%20%28single-precision%29))
  (Transformation|SetActorScale3D (Math|Vector|Lerp(Vector) (Variables|Default|GetLerpStartScale) "0, 0, 0" Alpha)))

(fn CrystalLightIntensity
  (params (Alpha :type Float%20%28single-precision%29))
  (Rendering|Components|Light|SetIntensity (Variables|Default|GetPointLight) (Math|Float|Lerp (Variables|Default|GetLerp%20Start%20Intensity) 0.0 Alpha)))