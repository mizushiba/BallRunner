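; BP_PlayerPawn is the player-controlled rolling ball pawn, with health and level restart on death.
; Movement axis inputs apply scaled torque to the Ball as acceleration change, and BeginPlay fades the camera in.
; AnyDamage subtracts from Health, which Tick polls.
; At zero or below, a DoOnce prints a message, starts a fade-out and reloads the current level after a short delay, before the fade finishes.
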(event EventBeginPlay
  (CameraFades|StartCameraFade :self (Game|GetPlayerCameraManager 0) :FromAlpha 1.0 :Duration 3.0))

(event EventTick
  (params (DeltaSeconds :type Float%20%28single-precision%29))
  (if (<= (Variables|Default|GetHealth) 0.0)
    (Utilities|FlowControl|DoOnce false
      (:Completed
        (Development|PrintString "0 health" true false "(R=1.000000,G=0.038177,B=0.000000,A=1.000000)" 0.5)
        (CameraFades|StartCameraFade :self (Game|GetPlayerCameraManager 0) :FromAlpha 0.0 :ToAlpha 1.0 :Duration 3.0)
        (Utilities|FlowControl|Delay 0.5)
        (bind _returnvalue (Game|GetCurrentLevelName true))
        (Game|OpenLevel(byName) (Utilities|String|StringToName _returnvalue))))))

(event Game|Damage|EventAnyDamage
  (params (Damage :type Float%20%28single-precision%29) (DamageType :type Damage%20Type%20Object%20Reference) (InstigatedBy :type Controller%20Object%20Reference) (DamageCauser :type Actor%20Object%20Reference))
  (Variables|Default|SetHealth (- (Variables|Default|GetHealth) Damage)))

(event Input|AxisEvents|InputAxisMoveForward/Back
  (params (AxisValue :type Float%20%28single-precision%29))
  (Class|PrimitiveComponent|AddTorqueinDegrees (Variables|Default|GetBall) (Math|Vector|MakeVector 0.0 (* AxisValue (Variables|Default|GetMultiply)) 0.0) "None" true))

(event Input|AxisEvents|InputAxisMoveLeft/Right
  (params (AxisValue :type Float%20%28single-precision%29))
  (Class|PrimitiveComponent|AddTorqueinDegrees (Variables|Default|GetBall) (Math|Vector|MakeVector (* AxisValue (Variables|Default|GetMultiply)) 0.0 0.0) "None" true))

(fn ConstructionScript)